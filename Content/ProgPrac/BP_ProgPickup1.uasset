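; BP_ProgPickup1 is a bobbing score pickup that the third-person character collects by overlapping it.
; A Timeline started on BeginPlay drives the sphere's vertical motion through its relative location.
; On overlap it finds the BP_ProgPrac actor, adds a small random amount to its Score, destroys itself and prints the new score.
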(event EventBeginPlay
  (bind _vertmovement (Timeline|Timeline Play)
    (:Update
      (Transformation|SetRelativeLocation (Variables|Default|GetSphere) (Math|Vector|MakeVector 0.0 0.0 (* _vertmovement 1e+02)) false false))))

(event Collision|EventActorBeginOverlap
  (params (OtherActor :type Actor%20Object%20Reference))
  (Utilities|Casting|CastToBP_ThirdPersonCharacter OtherActor)
  (bind _returnvalue (Actor|GetActorOfClass "/Game/ThirdPerson/Blueprints/BP_ProgPrac.BP_ProgPrac_C"))
  (bind _output_get (Variables|/Game/ThirdPerson/Blueprints/BP_ProgPrac.BP_ProgPrac_C|Setscore _returnvalue (+ (Variables|/Game/ThirdPerson/Blueprints/BP_ProgPrac.BP_ProgPrac_C|Getscore _returnvalue) (Math|Random|RandomIntegerinRange 5 10))))
  (Actor|DestroyActor)
  (Development|PrintString (Utilities|String|ToString(Integer) _output_get)))

(fn ConstructionScript)